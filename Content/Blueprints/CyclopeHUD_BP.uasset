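; HUD class for the Cyclope player that owns the on-screen PlayerHUDWidget and manages its health bar.
; On BeginPlay it creates the widget, adds it to the viewport and binds to CyclopePlayerController's possess and unpossess dispatchers.
; Those events show or hide the health bar as the pawn changes.
; An UpdateHealthBar event forwards the health alpha to the widget when it is valid.
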(event Custom|OnPawnPossessed_Event_0
  (Default|ToggleHealthBar (Variables|Default|GetMainWidget) true))

(event Custom|OnPawnUnPossessed_Event_0
  (Default|ToggleHealthBar (Variables|Default|GetMainWidget) false))

(event EventBeginPlay
  (bind _returnvalue (UserInterface|CreateWidget "/Game/Blueprints/UI/PlayerHUDWidget.PlayerHUDWidget_C" (Variables|Default|GetPlayerOwner)))
  (bind _output_get (Variables|Default|SetMainWidget _returnvalue))
  (UserInterface|Viewport|AddtoViewport _output_get 0)
  (bind _ascyclope_player_controller (Utilities|Casting|CastToCyclopePlayerController (Variables|Default|GetPlayerOwner)))
  (bind _output_get_2 (Variables|Default|SetAs%20Cyclope%20Player%20Controller _ascyclope_player_controller))
  (EventDispatchers|AssignOnPawnPossessed _output_get_2 (delegate Custom|OnPawnPossessed_Event_0))
  (EventDispatchers|AssignOnPawnUnPossessed _output_get_2 (delegate Custom|OnPawnUnPossessed_Event_0)))

(event EventUpdateHealthBar
  (params (HealthAlpha :type Float%20%28single-precision%29))
  (bind _mainwidget (Variables|Default|GetMainWidget)
    (:then
      (Default|UpdateHealthBar _mainwidget HealthAlpha))
    (:else)))

(fn ConstructionScript)